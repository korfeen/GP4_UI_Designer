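; Core HUD Blueprint that creates the game's UI widgets on BeginPlay and tracks most of them in a WidgetList array.
; HP, mana, hot bar, party, map, character profile and move-UI widgets are created and stored, but not added to the viewport here.
; A test movable-HUD widget receives this HUD and goes on screen, then is passed as drag-drop reference to the pause menu, also shown immediately.
; Disconnected scrapyard nodes duplicate earlier setup.
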(event EventBeginPlay
  (Utilities|FlowControl|Sequence
    (:then_0
      (bind _returnvalue (UserInterface|CreateWidget "/Game/UIDesigner/Widgets/WB_HP_Bar.WB_HP_Bar_C"))
      (bind _output_get (Variables|Default|SetHP%20bar _returnvalue))
      (Utilities|Array|Add (Variables|Default|GetWidgetList) _output_get)
      (bind _returnvalue_2 (UserInterface|CreateWidget "/Game/UIDesigner/Widgets/WB_MANA_Bar.WB_MANA_Bar_C"))
      (bind _output_get_2 (Variables|Default|SetMANA%20bar _returnvalue_2))
      (Utilities|Array|Add (Variables|Default|GetWidgetList) _output_get_2)
      (bind _returnvalue_3 (UserInterface|CreateWidget "/Game/UIDesigner/Widgets/WB_Hot_Bar.WB_Hot_Bar_C"))
      (bind _output_get_3 (Variables|Default|SetHOT%20bar _returnvalue_3))
      (Utilities|Array|Add (Variables|Default|GetWidgetList) _output_get_3)
      (bind _returnvalue_4 (UserInterface|CreateWidget "/Game/UIDesigner/Widgets/WB_Party.WB_Party_C"))
      (bind _output_get_4 (Variables|Default|SetParty%20bar _returnvalue_4))
      (Utilities|Array|Add (Variables|Default|GetWidgetList) _output_get_4)
      (bind _returnvalue_5 (UserInterface|CreateWidget "/Game/UIDesigner/Widgets/WB_MAP.WB_MAP_C"))
      (bind _output_get_5 (Variables|Default|SetMap%20icon _returnvalue_5))
      (Utilities|Array|Add (Variables|Default|GetWidgetList) _output_get_5)
      (bind _returnvalue_6 (UserInterface|CreateWidget "/Game/UIDesigner/Widgets/WB_CharacterProfile.WB_CharacterProfile_C"))
      (bind _output_get_6 (Variables|Default|SetCharacter%20Profile _returnvalue_6))
      (Utilities|Array|Add (Variables|Default|GetWidgetList) _output_get_6)
      (bind _returnvalue_7 (UserInterface|CreateWidget "/Game/UIDesigner/Widgets/WBP_MoveUI.WBP_MoveUI_C" 0 0))
      (bind _output_get_7 (Variables|Default|SetMoveUI _returnvalue_7))
      (Utilities|Array|Add (Variables|Default|GetWidgetList) _output_get_7))
    (:then_1
      ;[1 1 1] HUD start main UI
      (bind _returnvalue_8 (UserInterface|CreateWidget "/Game/UIDesigner/Widgets/TESTMOVEHUDCOOL.TESTMOVEHUDCOOL_C" (Variables|Default|GetOwning%20Player) self))
      (bind _output_get_8 (Variables|Default|SetHealthbar%20test _returnvalue_8))
      (UserInterface|Viewport|AddtoViewport _output_get_8 0))
    (:then_2
      ;[1 1 1] HUD.  Widget array start
      (bind _returnvalue_9 (UserInterface|CreateWidget "/Game/UIDesigner/Widgets/WB_Pause_menu.WB_Pause_menu_C" 0 (Variables|Default|GetHealthbar%20test)))
      (bind _output_get_9 (Variables|Default|SetPAUSE%20Menu _returnvalue_9))
      (Utilities|Array|Add (Variables|Default|GetWidgetList) _output_get_9)
      (UserInterface|Viewport|AddtoViewport _returnvalue_9 0))))

(fn ConstructionScript)