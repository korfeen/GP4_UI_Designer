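; Master NPC character that wanders or chases the player at a randomized walk speed, with a randomized outfit.
; When velocity reaches zero, Tick triggers a DoOnce-gated, randomly delayed move to the player or a nearby reachable point.
; The construction script has BPC_OutfitController randomize the look; the BeginPlay-style randomize call is unwired.
; Component-specific events that controller requires clear tagged meshes, assign materials by slot name and set morph targets.
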(event Custom|ClearComponents
  ;[1 0 0.004823] IMPORTANT: Component Specific, must be copied to your own character blueprint for BPC_OutfitController to operate
  (CallFunction|SetComponentArrays)
  (Utilities|FlowControl|Sequence
    (:then_0
      (for _array_element (Variables|Default|GetSkeletalMesh)
        (if (not (Components|ComponentHasTag _array_element "UE5Master"))
          (if (Components|ComponentHasTag _array_element "Parent")
            (Components|SkinnedMesh|SetSkinnedAssetandUpdate _array_element 0 true)
            (else
              (Components|DestroyComponent _array_element))))))
    (:then_1
      (for _array_element_2 (Variables|Default|GetStaticMesh)
        (Components|DestroyComponent _array_element_2)))))

(event Custom|SetComponentArrays
  ;[1 0 0.004823] IMPORTANT: Component Specific, must be copied to your own character blueprint for BPC_OutfitController to operate
  (Utilities|Array|Clear (Variables|Default|GetSkeletalMesh))
  (Utilities|Array|Clear (Variables|Default|GetStaticMesh))
  (Utilities|FlowControl|Sequence
    (:then_0
      (Variables|Default|SetSkeletalMesh (Actor|GetComponentsbyTag "/Script/Engine.SkeletalMeshComponent" "OutfitController"))
      (Utilities|Array|Add (Variables|Default|GetSkeletalMesh) (Utilities|Array|Get(acopy) (Actor|GetComponentsbyTag "/Script/Engine.SkeletalMeshComponent" "Parent"))))
    (:then_1
      (Variables|Default|SetStaticMesh (Actor|GetComponentsbyTag "/Script/Engine.StaticMeshComponent" "OutfitController")))))

(event Custom|SetMorphTarget
  (params (RandomValues :type Float%20%28double-precision%29))
  ;[1 0 0.004823] IMPORTANT: Component Specific, must be copied to your own character blueprint for BPC_OutfitController to operate
  (CallFunction|SetComponentArrays)
  (for _array_element (Variables|Default|GetSkeletalMesh)
    (bind _array_element_2 (Utilities|Array|ForEachLoopwithBreak (Variables|/Game/YI_NPC/Blueprints/Master/Components/BPC_OutfitController.BPC_OutfitController_C|GetMorphTargets (Variables|Default|GetAs%20BPC%20Outfit%20Controller)))
      (:LoopBody
        (for _array_element_3 (.MorphposeName (Utilities|Struct|BreakStruc_StaticMorphPoses _array_element_2))
          (Components|SkeletalMesh|SetMorphTarget _array_element (Utilities|String|StringToName _array_element_3) RandomValues true))))))

(event Custom|SetMaterials
  (params (SlotNames :type Array%20of%20Strings) (Materials :type Array%20of%20Material%20Instance%20Object%20References))
  ;[1 0 0.004823] IMPORTANT: Component Specific, must be copied to your own character blueprint for BPC_OutfitController to operate
  (CallFunction|SetComponentArrays)
  (for (_array_element _array_index) SlotNames
    (for _array_element_2 (Variables|Default|GetSkeletalMesh)
      ;;[1 1 1] Logic to make sure any duplicate slot names get assigned
      (for (_array_element_3 _array_index_2) (Class|MeshComponent|GetMaterialSlotNames _array_element_2)
        (if (== _array_element_3 (Utilities|String|StringToName _array_element))
          (Rendering|Material|SetMaterial _array_element_2 _array_index_2 (Utilities|Array|Get(acopy) Materials _array_index)))))))

(event Custom|MoveTo
  (bind _self self)
  (bind _returnvalue (AI|GetAIController _self))
  ;[0.1261 1 0] Basic AI logic
  (Utilities|FlowControl|Delay (Math|Random|RandomFloatinRange 0.0 3.0))
  (if (Variables|Default|GetChase)
    (AI|AIMoveTo _returnvalue "0, 0, 0" (Game|GetPlayerCharacter 0) -1.0 "Default" "Default" true true
      (:then
        (Utilities|FlowControl|DoOnce false) ; enters at Reset
      ))
    (else
      (AI|Navigation|MovetoLocation _returnvalue (.RandomLocation (AI|Navigation|GetRandomReachablePointinRadius (Transformation|GetActorLocation) 1e+03 0 0)) 2.5e+02 true true false true 0)
      (Utilities|FlowControl|DoOnce false) ; enters at Reset
    )))

(event EventTick
  (params (DeltaSeconds :type Float%20%28single-precision%29))
  ;[0.1261 1 0] Basic AI logic
  (if (Utilities|Operators|EqualEqual :A (Pawn|Components|CharacterMovement|GetLastUpdateVelocity (Variables|Character|GetCharacterMovement)))
    (Utilities|FlowControl|DoOnce false
      (:Completed
        (CallFunction|Moveto)))))

(event EventBeginPlay
  ;[0.09412 1 0] Randomize Walk Speed
  (Variables|/Script/Engine.CharacterMovementComponent|SetMaxWalkSpeed (Variables|Character|GetCharacterMovement) (Math|Random|RandomFloatinRange (Variables|Default|GetMinWalkSpeed) (Variables|Default|GetMaxWalkSpeed))))

(fn ConstructionScript
  (bind _output_get (Variables|Default|SetAs%20BPC%20Outfit%20Controller (Actor|GetComponentbyClass "/Game/YI_NPC/Blueprints/Master/Components/BPC_OutfitController.BPC_OutfitController_C")))
  (Default|RandomizeSelected _output_get))